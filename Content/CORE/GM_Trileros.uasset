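; Game mode for Trileros that runs the timed intro sequence, then starts play.
; BeginPlay caches the texts, game and camera pawn actors, plays music, and swaps title texts between timeline fades of a black sphere material's opacity.
; It then unhides SCENE-tagged actors and pawn circles, runs a final fade and calls Primerlevanta on BP_Juego.
; A separate NewTime event sets game speed through the slomo console command.
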(event Custom|FadePlane
  (bind _returnvalue (Rendering|Material|CreateDynamicMaterialInstance (Variables|/Game/CORE/BP_GameTexts.BP_GameTexts_C|GetSphere (Variables|Default|GetRef_Texts)) 0 "/Game/CORE/Materials/M_Black.M_Black" "None" :!class /Script/Engine.PrimitiveComponent))
  (bind _fade_value (Timeline|Fade PlayFromStart)
    (:Update
      (Rendering|Material|SetScalarParameterValue _returnvalue "Opa" _fade_value :!class /Script/Engine.MaterialInstanceDynamic))
    (:Finished
      (Utilities|FlowControl|Delay 4.0)
      (bind _returnvalue_2 (Rendering|Material|CreateDynamicMaterialInstance (Variables|/Game/CORE/BP_GameTexts.BP_GameTexts_C|GetSphere (Variables|Default|GetRef_Texts)) 0 "/Game/CORE/Materials/M_Black.M_Black" "None" :!class /Script/Engine.PrimitiveComponent))
      (bind _fade_value_2 (Timeline|Timeline_0 PlayFromStart)
        (:Update
          (Rendering|Material|SetScalarParameterValue _returnvalue_2 "Opa" _fade_value_2 :!class /Script/Engine.MaterialInstanceDynamic))))))

(event Custom|NewTime
  (params (Time :type Float%20%28single-precision%29))
  (Variables|Default|SetTime Time)
  (Development|ExecuteConsoleCommand (Utilities|String|Append "slomo" " " (Utilities|String|ToString(Float) (Variables|Default|GetTime))) 0))

(event EventBeginPlay
  (Utilities|FlowControl|Sequence
    (:then_0
      (bind _outactors (Actor|GetAllActorsOfClass "/Game/CORE/BP_GameTexts.BP_GameTexts_C"))
      (Variables|Default|SetRef_Texts (Utilities|Array|Get(acopy) _outactors))
      (bind _outactors_2 (Actor|GetAllActorsOfClass "/Game/CORE/BP_Juego.BP_Juego_C"))
      (Variables|Default|SetRef_Juego (Utilities|Array|Get(acopy) _outactors_2))
      (bind _outactors_3 (Actor|GetAllActorsOfClass "/Game/CORE/Pawn_CameraPico.Pawn_CameraPico_C"))
      (Variables|Default|SetRef_Pawn (Utilities|Array|Get(acopy) _outactors_3))
      (Audio|PlaySound2D "/Game/CORE/Audio/ElvenHarmonies.ElvenHarmonies" 1.0 1.0 0.0 0 0))
    (:then_1
      (Utilities|FlowControl|Delay 4.0)
      (CallFunction|FadePlane)
      (Utilities|FlowControl|Delay 8.0)
      (Rendering|SetVisibility (Variables|/Game/CORE/BP_GameTexts.BP_GameTexts_C|GetVivirtual (Variables|Default|GetRef_Texts)) false false)
      (Rendering|SetVisibility (Variables|/Game/CORE/BP_GameTexts.BP_GameTexts_C|GetLateOclock (Variables|Default|GetRef_Texts)) true false)
      (CallFunction|FadePlane)
      (Utilities|FlowControl|Delay 8.0)
      (bind _outactors_4 (Actor|GetAllActorswithTag "SCENE"))
      (for _array_element _outactors_4
        (Rendering|SetActorHiddenInGame _array_element false)
        (Rendering|SetVisibility (Variables|/Game/CORE/BP_GameTexts.BP_GameTexts_C|GetLateOclock (Variables|Default|GetRef_Texts)) false false)
        (Rendering|SetVisibility (Variables|/Game/CORE/BP_GameTexts.BP_GameTexts_C|Get01 (Variables|Default|GetRef_Texts)) true false)
        (bind _returnvalue (Rendering|Material|CreateDynamicMaterialInstance (Variables|/Game/CORE/BP_GameTexts.BP_GameTexts_C|GetSphere (Variables|Default|GetRef_Texts)) 0 "/Game/CORE/Materials/M_Black.M_Black" "None" :!class /Script/Engine.PrimitiveComponent))
        (bind _fade_value (Timeline|Timeline_1 PlayFromStart)
          (:Update
            (Rendering|Material|SetScalarParameterValue _returnvalue "Opa" _fade_value :!class /Script/Engine.MaterialInstanceDynamic))
          (:Finished
            (Default|Primerlevanta (Variables|Default|GetRef_Juego))))))))

(fn ConstructionScript)