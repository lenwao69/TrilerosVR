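; BP_Recompensa is a reward actor that displays an animal mesh and animates its scale shortly after spawning.
; On BeginPlay it checks the Animal code: ELE keeps the default mesh, while GAT, PER and DEL all use the Gato mesh, each with its own glass material instance.
; All four codes then share a short delay and a timeline that drives the mesh's world scale.
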(event EventBeginPlay
  (bind _staticmesh (Variables|Default|GetStaticMesh))
  (bind _staticmesh_2 (Variables|Default|GetStaticMesh))
  (bind _staticmesh_3 (Variables|Default|GetStaticMesh))
  (if (Utilities|Enum|Equal(Enum) (Variables|Default|GetAnimal) "ELE")
    (Utilities|FlowControl|Delay 1.0 :!label _label)
    (bind _scale (Timeline|Timeline_0 Play)
      (:Update
        (Transformation|SetWorldScale3D (Variables|Default|GetStaticMesh) (Math|Conversions|ToVector(Float) _scale))))
    (elif (Utilities|Enum|Equal(Enum) (Variables|Default|GetAnimal) "GAT")
      (Components|StaticMesh|SetStaticMesh _staticmesh_2 "/Game/CORE/Meshes/Gato.Gato")
      (Rendering|Material|SetMaterial _staticmesh_2 0 "/Game/CORE/Glass/MAT_Glass_Inst1.MAT_Glass_Inst1")
      (goto _label)
      (elif (Utilities|Enum|Equal(Enum) (Variables|Default|GetAnimal) "PER")
        (Components|StaticMesh|SetStaticMesh _staticmesh_3 "/Game/CORE/Meshes/Gato.Gato")
        (Rendering|Material|SetMaterial _staticmesh_3 0 "/Game/CORE/Glass/MAT_Glass_Inst2.MAT_Glass_Inst2")
        (goto _label)
        (elif (Utilities|Enum|Equal(Enum) (Variables|Default|GetAnimal) "DEL")
          (Components|StaticMesh|SetStaticMesh _staticmesh "/Game/CORE/Meshes/Gato.Gato")
          (Rendering|Material|SetMaterial _staticmesh 0 "/Game/CORE/Glass/MAT_Glass_Inst3.MAT_Glass_Inst3")
          (goto _label))))))

(fn ConstructionScript)