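; GM_Materials is a game mode for a materials test level that steps the player pawn through numbered camera positions.
; BeginPlay caches the player's Pawn_CameraPico.
; ChangeCamera advances a wrapping camera index, finds the Pawn_CameraPico actor tagged with that number, and copies its transform onto the player pawn, so placed pawns act as viewpoint markers.
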(event Custom|ChangeCamera
  (if (== (Variables|Default|GetActiveCamera) 10)
    (Variables|Default|SetActiveCamera 1)
    (else
      (Variables|Default|SetActiveCamera (+ (Variables|Default|GetActiveCamera) 1))))
  (bind _outactors (Actor|GetAllActorsOfClass "/Game/CORE/Pawn_CameraPico.Pawn_CameraPico_C"))
  (for _array_element _outactors
    (if (Actor|ActorHasTag _array_element (Utilities|String|StringToName (Utilities|String|ToString(Integer) (Variables|Default|GetActiveCamera))))
      (Transformation|SetActorTransform (Variables|Default|GetRef_Pawn) (Transformation|GetActorTransform _array_element)))))

(event EventBeginPlay
  (bind _aspawn_camera_pico (Utilities|Casting|CastToPawn_CameraPico (Game|Player|GetPlayerPawn 0)))
  (Variables|Default|SetRef_Pawn _aspawn_camera_pico))

(fn ConstructionScript)